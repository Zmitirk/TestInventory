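; Main player controller that creates and shows the HUD and inventory widgets for the player.
; On possess it creates WBP_HUD once and makes it visible, and the OpenInventory input lazily creates and shows WBP_Inventory with a mouse cursor and UI-only input.
; RemoveInventory hides the inventory and cursor without restoring game input mode, and both open and close fire OnInventoryOpened/Closed notifications.
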(event Custom|DisplayInventory
  (Utilities|IsValid (Variables|Default|GetInventoryWidget)
    (:Is%20Valid
      _)
    (:Is%20Not%20Valid
      (bind _returnvalue (UserInterface|CreateWidget "/Game/Widgets/WBP_Inventory.WBP_Inventory_C" self))
      (Variables|Default|SetInventoryWidget _returnvalue)
      (UserInterface|Viewport|AddtoViewport (Variables|Default|GetInventoryWidget) 0)))
  (Widget|SetVisibility (Variables|Default|GetInventoryWidget) "Visible")
  (Variables|Default|SetbShowMouseCursor true)
  (Input|SetInputModeUIOnly self (Variables|Default|GetInventoryWidget) "DoNotLock")
  (Default|CallOnInventoryOpened))

(event Custom|RemoveInventory
  (bind _inventorywidget (Variables|Default|GetInventoryWidget))
  (Utilities|IsValid _inventorywidget
    (:Is%20Valid
      (Widget|SetVisibility _inventorywidget "Hidden")
      (Variables|Default|SetbShowMouseCursor false)
      (Default|CallOnInventoryClosed))))

(event EventPossess
  (params (PossessedPawn :type Pawn%20Object%20Reference))
  (Utilities|IsValid (Variables|Default|GetHUDWidget)
    (:Is%20Valid
      _)
    (:Is%20Not%20Valid
      (bind _returnvalue (UserInterface|CreateWidget "/Game/Widgets/WBP_HUD.WBP_HUD_C" self))
      (bind _output_get (Variables|Default|SetHUDWidget _returnvalue))
      (UserInterface|Viewport|AddtoViewport _output_get 0)))
  (Widget|SetVisibility (Variables|Default|GetHUDWidget) "Visible"))

(event Input|ActionEvents|InputActionOpenInventory
  (params (Key :type Key%20Structure :default "None"))
  (:Pressed
    (CallFunction|DisplayInventory)))

(fn ConstructionScript)