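; Base weapon inventory item that equips itself on the third-person character when used.
; If a weapon is already equipped, it returns that weapon's item to the inventory and destroys its actor first, doing nothing if that item is invalid.
; It spawns a BP_WeaponEquipped with the item's pickup mesh, ignores collision and attaches the mesh to WeaponSocket.
; The spawned actor references this item, whose quantity becomes one.
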(event EventOnUse
  (params (Character :type Test%20Project%20Character%20Object%20Reference))
  (bind _asbp_third_person_character (Utilities|Casting|CastToBP_ThirdPersonCharacter Character))
  (bind _output_get (Variables|Default|SetAs%20BP%20Third%20Person%20Character _asbp_third_person_character))
  (if (Variables|/Game/Blueprints/BP_ThirdPersonCharacter.BP_ThirdPersonCharacter_C|GetIsWeaponEquipped _output_get)
    (Utilities|IsValid (Variables|/Game/Blueprints/BP_WeaponEquipped.BP_WeaponEquipped_C|GetItem (Variables|/Game/Blueprints/BP_ThirdPersonCharacter.BP_ThirdPersonCharacter_C|GetEquippedWeapon (Variables|Default|GetAs%20BP%20Third%20Person%20Character)))
      (:Is%20Valid
        (Class|InventoryComponent|TryAddItem (Variables|/Script/TestProject.TestProjectCharacter|GetPlayerInventory (Variables|Default|GetAs%20BP%20Third%20Person%20Character)) (Variables|/Game/Blueprints/BP_WeaponEquipped.BP_WeaponEquipped_C|GetItem (Variables|/Game/Blueprints/BP_ThirdPersonCharacter.BP_ThirdPersonCharacter_C|GetEquippedWeapon (Variables|Default|GetAs%20BP%20Third%20Person%20Character))))
        (Actor|DestroyActor (Variables|/Game/Blueprints/BP_ThirdPersonCharacter.BP_ThirdPersonCharacter_C|GetEquippedWeapon (Variables|Default|GetAs%20BP%20Third%20Person%20Character)))
        (CallFunction|EquipeWeapon (Variables|Default|GetAs%20BP%20Third%20Person%20Character))))
    (else
      (CallFunction|EquipeWeapon _output_get))))

(fn EquipeWeapon
  (params (Character :type BP%20Third%20Person%20Character%20Object%20Reference))
  (bind _mesh (Variables|/Script/Engine.Character|GetMesh Character))
  (bind _skeletalmesh (Variables|/Script/Engine.SkinnedMeshComponent|GetSkeletalMesh _mesh))
  (bind _returnvalue (Class|SkeletalMesh|FindSocket _skeletalmesh "WeaponSocket"))
  (bind _returnvalue_2 (Game|SpawnActorfromClass "/Game/Blueprints/BP_WeaponEquipped.BP_WeaponEquipped_C" (Math|Transform|MakeTransform (Variables|/Script/Engine.SkeletalMeshSocket|GetRelativeLocation _returnvalue) (Variables|/Script/Engine.SkeletalMeshSocket|GetRelativeRotation _returnvalue)) "Undefined" 0 Character))
  (CallFunction|SetAttributes _returnvalue_2)
  (Variables|/Game/Blueprints/BP_ThirdPersonCharacter.BP_ThirdPersonCharacter_C|SetIsWeaponEquipped Character true)
  (Variables|/Game/Blueprints/BP_ThirdPersonCharacter.BP_ThirdPersonCharacter_C|SetEquippedWeapon Character _returnvalue_2))

(fn SetAttributes
  (params (SpawnedActor :type BP%20Weapon%20Equipped%20Object%20Reference))
  (Components|StaticMesh|SetStaticMesh (Variables|/Game/Blueprints/BP_WeaponEquipped.BP_WeaponEquipped_C|GetStaticMesh SpawnedActor) (Variables|Default|GetPickupMesh self))
  (Collision|SetCollisionResponsetoAllChannels (Variables|/Game/Blueprints/BP_WeaponEquipped.BP_WeaponEquipped_C|GetStaticMesh SpawnedActor) "ECR_Ignore")
  (Transformation|AttachComponentToComponent (Variables|/Game/Blueprints/BP_WeaponEquipped.BP_WeaponEquipped_C|GetStaticMesh SpawnedActor) (Variables|/Script/Engine.Character|GetMesh (Variables|Default|GetAs%20BP%20Third%20Person%20Character)) "WeaponSocket" "KeepRelative" "KeepRelative" "KeepRelative" true)
  (bind _output_get (Variables|/Game/Blueprints/BP_WeaponEquipped.BP_WeaponEquipped_C|SetItem SpawnedActor self))
  (Class|Item|SetQuantity _output_get 1))